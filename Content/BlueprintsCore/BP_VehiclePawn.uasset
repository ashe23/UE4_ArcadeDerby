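; BP_VehiclePawn is a physics-driven vehicle pawn that attempts a simple hover suspension at four wheel points.
; Each tick, it line-traces down from each wheel and pushes VehicleMesh with a fixed force at that point, down above a height threshold, otherwise up.
; Traces, wheel points and heights are shown as debug output.
; MoveVehicle applies a given direction to the mesh as a mass-independent force.
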(event `self.ReceiveTick`
  (params (DeltaSeconds :type "Float (single-precision)"))
  (bind _vehiclemesh (`self.VehicleMesh`))
  (for _array_element (`|MakeArray` (`self.WheelFL`) (`self.WheelFR`) (`self.WheelRL`) (`self.WheelRR`))
    (bind _returnvalue (`SceneComponent.K2_GetComponentLocation` _array_element))
    (bind _outhit (`KismetSystemLibrary.LineTraceSingle` :`Start` _returnvalue :`End` (- _returnvalue (0.0 0.0 500.0)) :`TraceChannel` "TraceTypeQuery1" :`DrawDebugType` "ForDuration" :`DrawTime` 1.0))
    (bind _output_get (set `self.Height` (`KismetMathLibrary.VSize` (- (`.Location` (`GameplayStatics.BreakHitResult` _outhit)) _returnvalue))))
    (`KismetSystemLibrary.PrintString` (`KismetStringLibrary.Conv_DoubleToString` _output_get) true false (struct :`G` 0.66 :`B` 1.0 :`A` 1.0) 0.0)
    (`KismetSystemLibrary.DrawDebugPoint` _returnvalue 4.0 (struct :`R` 1.0 :`A` 1.0))
    (if (> _output_get 100.0)
      (`PrimitiveComponent.AddForceAtLocation` _vehiclemesh (0.0 0.0 -300.0) _returnvalue "None")
      (else
        (`PrimitiveComponent.AddForceAtLocation` _vehiclemesh (0.0 0.0 300.0) _returnvalue "None")))))

(fn `MoveVehicle`
  (params (Direction :type "Vector Structure"))
  (`PrimitiveComponent.AddForce` (`self.VehicleMesh`) Direction "None" true))

(fn `UserConstructionScript`)